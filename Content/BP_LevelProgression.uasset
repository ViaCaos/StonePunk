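; BP_LevelProgression is a level-exit trigger that moves the game on to the next map when the player touches it.
; On BeginPlay it picks NextLevel from a hardcoded chain keyed on the current level name: FirstPersonMap to Segunda_Fase, then to fase_boss.
; Its Box overlap opens NextLevel by name, only for player 0's character.
; Any other map leaves NextLevel at its default value.
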(event `self.Box.OnComponentBeginOverlap`
  (params (OverlappedComponent :type "PrimitiveComponent Object Reference") (OtherActor :type "Actor Object Reference") (OtherComp :type "PrimitiveComponent Object Reference") (OtherBodyIndex :type Integer) (bFromSweep :type Boolean) (SweepResult :type "HitResult Structure (by ref)"))
  (`/Engine/EditorBlueprintResources/StandardMacros.IsValid` OtherActor
    (:`Is Valid`
      (if (== OtherActor (`GameplayStatics.GetPlayerCharacter` 0))
        (`GameplayStatics.OpenLevel` (`KismetStringLibrary.Conv_StringToName` (`self.NextLevel`)))))))

(event `self.ReceiveBeginPlay`
  (bind _returnvalue (`GameplayStatics.GetCurrentLevelName` true))
  (if (`KismetStringLibrary.EqualEqual_StrStr` _returnvalue "FirstPersonMap")
    (set `self.NextLevel` "Segunda_Fase")
    (elif (`KismetStringLibrary.EqualEqual_StrStr` _returnvalue "Segunda_Fase")
      (set `self.NextLevel` "fase_boss"))))

(fn `UserConstructionScript`)