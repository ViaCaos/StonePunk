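; BP_Boss is the boss enemy, whose defeat sends the game back to the main menu level.
; Tick copies HitPoints into its AI controller's Blackboard every frame.
; Damage reduces HitPoints, then a timed flag ignores further hits for a short window.
; A RotatetoPlayer event turns the boss toward the player with pitch zeroed to keep it upright.
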(event `self.ReceiveBeginPlay`)

(event `self.ReceiveTick`
  (params (DeltaSeconds :type "Float (single-precision)"))
  (`BlackboardComponent.SetValueAsInt` (`AIBlueprintHelperLibrary.GetBlackboard` (`self.GetController`)) "HitPoints" (`self.HitPoints`)))

(event `/Game/Enemy/Boss/Blueprints/BPI_Boss.RotateToPlayer`
  (`self.K2_SetActorRotation` (`KismetMathLibrary.MakeRotator` (.roll (`KismetMathLibrary.FindLookAtRotation` (`self.K2_GetActorLocation`) (`self.K2_GetActorLocation` (`GameplayStatics.GetPlayerPawn` 0)))) 0.0 (.yaw (`KismetMathLibrary.FindLookAtRotation` (`self.K2_GetActorLocation`) (`self.K2_GetActorLocation` (`GameplayStatics.GetPlayerPawn` 0)))))))

(event `self.ReceiveAnyDamage`
  (params (Damage :type "Float (single-precision)") (DamageType :type "DamageType Object Reference") (InstigatedBy :type "Controller Object Reference") (DamageCauser :type "Actor Object Reference"))
  (if (not (`self.bIsTakingDmg`))
    (set `self.bIsTakingDmg` true)
    (set `self.HitPoints` (`KismetMathLibrary.FTrunc` (- (`self.HitPoints`) Damage)))
    (if (<= (`self.HitPoints`) 0)
      (`GameplayStatics.OpenLevel` "mainmenu_level")
      (else
        (`KismetSystemLibrary.K2_SetTimerDelegate` (delegate `ResetDmg`) 2.0)))))

(event `ResetDmg`
  (set `self.bIsTakingDmg` false))

(fn `UserConstructionScript`)