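; Boss behavior tree task that turns toward the player, then charges along that direction.
; Tick rotates the pawn and writes player location to the TargetLocation blackboard key until a delayed StartedAttack flag locks it.
; A navigation raycast to five times the target offset supplies the AIMoveTo destination; after a pause, the task finishes with the move's result.
; Debug drawing, printing, an unused line trace and disconnected overlap checks remain.
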(event `self.ReceiveExecuteAI`
  (params (OwnerController :type "AIController Object Reference") (ControlledPawn :type "Pawn Object Reference"))
  (bind _returnvalue (`Actor.K2_GetActorLocation` ControlledPawn))
  (bind _returnvalue_2 (+ (* (- (`BlackboardComponent.GetValueAsVector` (`AIBlueprintHelperLibrary.GetBlackboard` ControlledPawn) "TargetLocation") _returnvalue) 5) _returnvalue))
  (`KismetSystemLibrary.Delay` 4.0)
  (set `self.bStartedAttack` true)
  (`KismetSystemLibrary.Delay` 2.0)
  (`KismetSystemLibrary.DrawDebugLine` _returnvalue _returnvalue_2 (struct :`R` 1.0 :`A` 1.0) 20.0 20.0)
  (bind _outhit (`KismetSystemLibrary.LineTraceSingleForObjects` :`Start` _returnvalue :`End` _returnvalue_2 :`ObjectTypes` (`|MakeArray` "ObjectTypeQuery1" :!type "EObjectTypeQuery Enum") :`DrawDebugType` "Persistent" :`DrawTime` 10.0))
  (`KismetSystemLibrary.DrawDebugSphere` (stale _hitlocation) 200.0 12 (struct :`R` 1.0 :`G` 1.0 :`B` 1.0 :`A` 1.0) 10.0 10.0)
  (bind _hitlocation (`NavigationSystemV1.NavigationRaycast` (`NavigationSystemV1.GetNavigationSystem`) _returnvalue _returnvalue_2 "/Script/AIModule.NavFilter_AIControllerDefault" null))
  (`KismetSystemLibrary.PrintString` (`KismetStringLibrary.Conv_VectorToString` _hitlocation))
  (bind _movementresult (`|AIMoveTo` ControlledPawn _hitlocation null)
    (:`OnSuccess`
      (`KismetSystemLibrary.Delay` 5.0)
      (set `self.bStartedAttack` false)
      (`self.FinishExecute` true))
    (:`OnFail`
      (`KismetSystemLibrary.Delay` 5.0)
      (set `self.bStartedAttack` false)
      (`self.FinishExecute` false))))

(event `self.ReceiveTickAI`
  (params (OwnerController :type "AIController Object Reference") (ControlledPawn :type "Pawn Object Reference") (DeltaSeconds :type "Float (single-precision)"))
  (if (not (`self.bStartedAttack`))
    (message `/Game/Enemy/Boss/Blueprints/BPI_Boss.RotateToPlayer` ControlledPawn)
    (`BTFunctionLibrary.SetBlackboardValueAsVector` (make `BlackboardKeySelector` :`SelectedKeyName` "TargetLocation" :`SelectedKeyType` "/Script/AIModule.BlackboardKeyType_Vector") (`Actor.K2_GetActorLocation` (`GameplayStatics.GetPlayerCharacter` 0)))))