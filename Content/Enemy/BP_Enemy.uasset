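; Enemy that spots the player through PawnSensing, turns to face them, chases them and damages them on contact.
; A StartMovement dispatcher runs AI MoveTo and re-fires itself on each success while the enemy is alive.
; DamageHitbox overlaps call the player's TakeDamage, ignoring the InteractRadius component.
; The Kill dispatcher marks it dead and destroys the hitbox, with Detected and Dead states pushed to ABP_chupacu2.
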(event `self.ReceiveTick`
  (params (DeltaSeconds :type "Float (single-precision)"))
  (if (`KismetSystemLibrary.IsValid` (`self.Target`))
    (if (`self.bAlive`)
      (`self.K2_SetActorRotation` (`KismetMathLibrary.MakeRotator` (.roll (`KismetMathLibrary.FindLookAtRotation` (`self.K2_GetActorLocation`) (`self.K2_GetActorLocation` (`GameplayStatics.GetPlayerPawn` 0)))) 0.0 (.yaw (`KismetMathLibrary.FindLookAtRotation` (`self.K2_GetActorLocation`) (`self.K2_GetActorLocation` (`GameplayStatics.GetPlayerPawn` 0)))))))))

(event `self.PawnSensing.OnSeePawn`
  (params (Pawn :type "Pawn Object Reference"))
  (if (== Pawn (`GameplayStatics.GetPlayerCharacter` 0))
    (set `self.Target` Pawn)
    (`self.UpdateAnimVar` false true)))

(event `StartMovement_Event`
  (`|AIMoveTo` self (0.0 0.0 0.0) (`self.Target`)
    (:`OnSuccess`
      (if (`self.bAlive`)
        (`self.StartMovement`)))))

(event `self.ReceiveBeginPlay`
  (add `self.Kill` (delegate `Kill_Event`))
  (add `self.StartMovement` (delegate `StartMovement_Event`)))

(event `Kill_Event`
  (if (`self.bAlive`)
    (set `self.bAlive` false)
    (`self.UpdateAnimVar` true)
    (`ActorComponent.K2_DestroyComponent` (`self.DamageHitbox`))))

(event `self.DamageHitbox.OnComponentBeginOverlap`
  (params (OverlappedComponent :type "PrimitiveComponent Object Reference") (OtherActor :type "Actor Object Reference") (OtherComp :type "PrimitiveComponent Object Reference") (OtherBodyIndex :type Integer) (bFromSweep :type Boolean) (SweepResult :type "HitResult Structure (by ref)"))
  (`/Engine/EditorBlueprintResources/StandardMacros.IsValid` OtherActor
    (:`Is Valid`
      (if (== OtherActor (`GameplayStatics.GetPlayerCharacter` 0))
        (bind _asbp_first_person_character (cast `/Game/FirstPerson/Blueprints/BP_FirstPersonCharacter` (`GameplayStatics.GetPlayerCharacter` 0)))
        (if (not (== OtherComp (`/Game/FirstPerson/Blueprints/BP_FirstPersonCharacter.InteractRadius` _asbp_first_person_character)))
          (`/Game/FirstPerson/Blueprints/BP_FirstPersonCharacter.TakeDamage` _asbp_first_person_character self))))))

(fn `UpdateAnimVar`
  (params (bDead :type Boolean) (bDetected :type Boolean))
  (bind _asabp_chupacu_2 (cast `/Game/Enemy/ABP_chupacu2` (`SkeletalMeshComponent.GetAnimInstance` (`self.Mesh`))))
  (if bDead
    (set `/Game/Enemy/ABP_chupacu2.bDead` true _asabp_chupacu_2)
    (return)
    (elif bDetected
      (set `/Game/Enemy/ABP_chupacu2.bDetected` true _asabp_chupacu_2)
      (return))))

(fn `UserConstructionScript`)