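; Dialogue asset for a terrified NPC ("Aterrorizado") who urges the player in Portuguese to flee from deadly creatures of unknown origin.
; Overrides the parent Dialogue function with one tree at index 0, built from nested AddDialogue calls that branch on the chosen option.
; Every ending closes the dialogue after clearing progress, except the "those who tried died" branch, which calls RemoveDialogueProgress(1) instead.
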(fn `Dialogue`
  (`parent.Dialogue`)
  (switch `int` (`self.DialogueTreeIndex`)
    (:`0`
      (bind (_state _optionindex) (`self.AddDialogue` "Aterrorizado" "Fuja! Fuja! FUJA!!" (`|MakeArray` "Para onde?" "Mas aqui não seguro?" :!type "Text")))
      (switch `/Game/Dialogue/Blueprints/Enum_DialogueState` _state
        (:`NewEnumerator0`
          (switch `int` _optionindex
            (:`0`
              (bind (_state_2 _optionindex_2) (`self.AddDialogue` "Aterrorizado" "Para algum lugar longe..... ELES vieram distante....lugar" (`|MakeArray` "Quem?" "Que lugar?" :!type "Text")))
              (switch `/Game/Dialogue/Blueprints/Enum_DialogueState` _state_2
                (:`NewEnumerator0`
                  (switch `int` _optionindex_2
                    (:`0`
                      (bind _state_3 (`self.AddDialogue` "Aterrorizado" "Como QUEM? Os BIXOS!" (`|MakeArray` "Encerrar Dialogo" :!type "Text")))
                      (switch `/Game/Dialogue/Blueprints/Enum_DialogueState` _state_3
                        (:`NewEnumerator0`
                          (`self.ClearDialogueProgress`)
                          (`self.CloseDialogue`))))
                    (:`1`
                      (bind (_state_4 _optionindex_3) (`self.AddDialogue` "Aterrorizado" "Não sabe... Nenhum sabe, apareceram um dia.... Mataram muitos" (`|MakeArray` "E depois...?" "Nunca foi atrás saber?" :!type "Text")))
                      (switch `/Game/Dialogue/Blueprints/Enum_DialogueState` _state_4
                        (:`NewEnumerator0`
                          (switch `int` _optionindex_3
                            (:`0`
                              (bind _state_5 (`self.AddDialogue` "Aterrorizado" "Todos junto aqui....Tentar sobrevivência.....Falha....FUJA " (`|MakeArray` "Encerrar Dialogo" :!type "Text")))
                              (switch `/Game/Dialogue/Blueprints/Enum_DialogueState` _state_5
                                (:`NewEnumerator0`
                                  (`self.ClearDialogueProgress`)
                                  (`self.CloseDialogue`))))
                            (:`1`
                              (bind _state_6 (`self.AddDialogue` "Aterrorizado" "Todos que tentaram..... morte" (`|MakeArray` "Encerrar Diálogo" :!type "Text")))
                              (switch `/Game/Dialogue/Blueprints/Enum_DialogueState` _state_6
                                (:`NewEnumerator0`
                                  (`self.RemoveDialogueProgress` 1)
                                  (`self.CloseDialogue`))))))))))))
            (:`1`
              (bind _state_7 (`self.AddDialogue` "Aterrorizado" "AH ! NENHUM LUGAR" (`|MakeArray` "Encerrar diálogo" :!type "Text")))
              (switch `/Game/Dialogue/Blueprints/Enum_DialogueState` _state_7
                (:`NewEnumerator0`
                  (`self.ClearDialogueProgress`)
                  (`self.CloseDialogue`))))))))))