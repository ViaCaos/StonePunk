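; Dialogue component for Zé3, a terrified character ("Aterrorizado") who warns the player in Portuguese about descending to the horrors below.
; It overrides the parent Dialogue function, calls it, then builds a single conversation for tree index 0 from nested AddDialogue nodes branching on OptionIndex.
; Each branch ends by clearing dialogue progress and closing the dialogue.
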(fn `Dialogue`
  (`parent.Dialogue`)
  (switch `int` (`self.DialogueTreeIndex`)
    (:`0`
      (bind (_state _optionindex) (`self.AddDialogue` "Aterrorizado" "Certeza vai descer?" (`|MakeArray` "O que tem embaixo" "Sim" :!type "Text")))
      (switch `/Game/Dialogue/Blueprints/Enum_DialogueState` _state
        (:`NewEnumerator0`
          (switch `int` _optionindex
            (:`0`
              (bind (_state_2 _optionindex_2) (`self.AddDialogue` "Aterrorizado" "Mais horror? Mais morte? Não sabe....MEDO" (`|MakeArray` "Devo voltar?" "Ninguém desceu?" :!type "Text")))
              (switch `/Game/Dialogue/Blueprints/Enum_DialogueState` _state_2
                (:`NewEnumerator0`
                  (switch `int` _optionindex_2
                    (:`0`
                      (bind _state_3 (`self.AddDialogue` "Aterrorizado" "FUJA" (`|MakeArray` "Encerrar Dialogo" :!type "Text")))
                      (switch `/Game/Dialogue/Blueprints/Enum_DialogueState` _state_3
                        (:`NewEnumerator0`
                          (`self.ClearDialogueProgress`)
                          (`self.CloseDialogue`))))
                    (:`1`
                      (bind (_state_4 _optionindex_3) (`self.AddDialogue` "Aterrorizado" "Alguns....ninguém voltou....provavelmente mortos" (`|MakeArray` "Mais monstros embaixo?" "Me deseje sorte" :!type "Text")))
                      (switch `/Game/Dialogue/Blueprints/Enum_DialogueState` _state_4
                        (:`NewEnumerator0`
                          (switch `int` _optionindex_3
                            (:`0`
                              (bind _state_5 (`self.AddDialogue` "Aterrorizado" "Mais escuro, mais bixo, outro bixo.....outro bixo? AH!" (`|MakeArray` "Encerrar Dialogo" :!type "Text")))
                              (switch `/Game/Dialogue/Blueprints/Enum_DialogueState` _state_5
                                (:`NewEnumerator0`
                                  (`self.ClearDialogueProgress`)
                                  (`self.CloseDialogue`))))
                            (:`1`
                              (bind _state_6 (`self.AddDialogue` "Aterrorizado" "Não....Nem Deus pode te salvar....." (`|MakeArray` "Encerrar Diálogo" :!type "Text")))
                              (switch `/Game/Dialogue/Blueprints/Enum_DialogueState` _state_6
                                (:`NewEnumerator0`
                                  (`self.ClearDialogueProgress`)
                                  (`self.CloseDialogue`))))))))))))
            (:`1`
              (bind _state_7 (`self.AddDialogue` "Aterrorizado" "Boa sorte" (`|MakeArray` "Encerrar diálogo" :!type "Text")))
              (switch `/Game/Dialogue/Blueprints/Enum_DialogueState` _state_7
                (:`NewEnumerator0`
                  (`self.ClearDialogueProgress`)
                  (`self.CloseDialogue`))))))))))