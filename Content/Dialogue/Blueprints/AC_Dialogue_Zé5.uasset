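; Dialogue component for the NPC Zé, a strange man ("Homem estranho") who talks in Portuguese about being lost and about a creature that wiped out most of his group.
; It overrides Dialogue, switching on DialogueTreeIndex, with a single tree defined at index 0.
; Nested AddDialogue calls branch on the chosen option index, and every ending clears dialogue progress and closes the dialogue.
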(fn `Dialogue`
  (`parent.Dialogue`)
  (switch `int` (`self.DialogueTreeIndex`)
    (:`0`
      (bind (_state _optionindex) (`self.AddDialogue` "Homem estranho" "Você se perdeu também?" (`|MakeArray` "Eu sei onde estou indo..." "Como faço para voltar?" :!type "Text")))
      (switch `/Game/Dialogue/Blueprints/Enum_DialogueState` _state
        (:`NewEnumerator0`
          (switch `int` _optionindex
            (:`0`
              (bind (_state_2 _optionindex_2) (`self.AddDialogue` "Homem estranho" "O que fazer? Vai matar a coisa?" (`|MakeArray` "Irei salvar todos nós" "Ela é muito forte?" :!type "Text")))
              (switch `/Game/Dialogue/Blueprints/Enum_DialogueState` _state_2
                (:`NewEnumerator0`
                  (switch `int` _optionindex_2
                    (:`0`
                      (bind _state_3 (`self.AddDialogue` "Homem estranho" "Você coragem ou apenas burro?" (`|MakeArray` "Encerrar Dialogo" :!type "Text")))
                      (switch `/Game/Dialogue/Blueprints/Enum_DialogueState` _state_3
                        (:`NewEnumerator0`
                          (`self.ClearDialogueProgress`)
                          (`self.CloseDialogue`))))
                    (:`1`
                      (bind (_state_4 _optionindex_3) (`self.AddDialogue` "Homem estranho" "O que acha? Tinham muitos de nós, agora só o que restou foram os que já perderam tudo" (`|MakeArray` "Em quantos vocês eram?" "Eu sinto muito" :!type "Text")))
                      (switch `/Game/Dialogue/Blueprints/Enum_DialogueState` _state_4
                        (:`NewEnumerator0`
                          (switch `int` _optionindex_3
                            (:`0`
                              (bind _state_5 (`self.AddDialogue` "Homem estranho" "Morávamos vários lugares, viemos procurando abrigo, nada mais agora..." (`|MakeArray` "Encerrar Dialogo" :!type "Text")))
                              (switch `/Game/Dialogue/Blueprints/Enum_DialogueState` _state_5
                                (:`NewEnumerator0`
                                  (`self.ClearDialogueProgress`)
                                  (`self.CloseDialogue`))))
                            (:`1`
                              (bind _state_6 (`self.AddDialogue` "Homem estranho" "Sinta por você" (`|MakeArray` "Encerrar Diálogo" :!type "Text")))
                              (switch `/Game/Dialogue/Blueprints/Enum_DialogueState` _state_6
                                (:`NewEnumerator0`
                                  (`self.ClearDialogueProgress`)
                                  (`self.CloseDialogue`))))))))))))
            (:`1`
              (bind _state_7 (`self.AddDialogue` "Homem estranho" "Também não sabemos..." (`|MakeArray` "Encerrar diálogo" :!type "Text")))
              (switch `/Game/Dialogue/Blueprints/Enum_DialogueState` _state_7
                (:`NewEnumerator0`
                  (`self.ClearDialogueProgress`)
                  (`self.CloseDialogue`))))))))))