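; Dialogue component for the NPC Zé, holding his branching Portuguese conversation with player reply options.
; The Dialogue override switches on the tree index, then chains AddDialogue calls that branch on the chosen option once each passes through.
; Apologizing moves the tree to a friendlier follow-up line; endings clear progress, except the stubborn reply, which removes progress before closing.
; Debug prints show the option and tree index.
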(fn `Dialogue`
  (`parent.Dialogue`)
  (switch `int` (`self.DialogueTreeIndex`)
    (:`0`
      (bind (_state _optionindex) (`self.AddDialogue` "Zé" "Olá nerd!!" (`|MakeArray` "Morra" "Me matei" :!type "Text")))
      (`KismetSystemLibrary.PrintText` (`KismetTextLibrary.Conv_IntToText` _optionindex))
      (`KismetSystemLibrary.PrintText` (`KismetTextLibrary.Conv_IntToText` (`self.DialogueTreeIndex`)))
      (switch `/Game/Dialogue/Blueprints/Enum_DialogueState` _state
        (:`NewEnumerator0`
          (switch `int` _optionindex
            (:`0`
              (bind (_state_2 _optionindex_2) (`self.AddDialogue` "Zé" "Não" (`|MakeArray` "Aff" "Ti fude" :!type "Text")))
              (switch `/Game/Dialogue/Blueprints/Enum_DialogueState` _state_2
                (:`NewEnumerator0`
                  (switch `int` _optionindex_2
                    (:`0`
                      (bind _state_3 (`self.AddDialogue` "Zé" "Hihi" (`|MakeArray` "Encerrar Dialogo" :!type "Text")))
                      (switch `/Game/Dialogue/Blueprints/Enum_DialogueState` _state_3
                        (:`NewEnumerator0`
                          (`self.ClearDialogueProgress`)
                          (`self.CloseDialogue`))))
                    (:`1`
                      (bind (_state_4 _optionindex_3) (`self.AddDialogue` "Zé" "Agora pede desculpa" (`|MakeArray` "mb dog" "Nao" :!type "Text")))
                      (switch `/Game/Dialogue/Blueprints/Enum_DialogueState` _state_4
                        (:`NewEnumerator0`
                          (switch `int` _optionindex_3
                            (:`0`
                              (bind _state_5 (`self.AddDialogue` "Zé" "Tmj ent" (`|MakeArray` "Encerrar Dialogo" :!type "Text")))
                              (switch `/Game/Dialogue/Blueprints/Enum_DialogueState` _state_5
                                (:`NewEnumerator0`
                                  (`self.SetDialogueTreeIndex` 1)
                                  (`self.ClearDialogueProgress`)
                                  (`self.CloseDialogue`))))
                            (:`1`
                              (bind _state_6 (`self.AddDialogue` "Zé" "Gente teimosa nao presta" (`|MakeArray` "Continuar" :!type "Text")))
                              (switch `/Game/Dialogue/Blueprints/Enum_DialogueState` _state_6
                                (:`NewEnumerator0`
                                  (`self.RemoveDialogueProgress` 1)
                                  (`self.CloseDialogue`))))))))))))
            (:`1`
              (bind _state_7 (`self.AddDialogue` "Zé" "Que isso meu filho calma" (`|MakeArray` "Gozei" :!type "Text")))
              (switch `/Game/Dialogue/Blueprints/Enum_DialogueState` _state_7
                (:`NewEnumerator0`
                  (`self.ClearDialogueProgress`)
                  (`self.CloseDialogue`))))))))
    (:`1`
      (bind _state_8 (`self.AddDialogue` "Zé" "Vc eh d boa dog" (`|MakeArray` "Encerrar Dialogo" :!type "Text")))
      (switch `/Game/Dialogue/Blueprints/Enum_DialogueState` _state_8
        (:`NewEnumerator0`
          (switch `int` 0
            (:`0`
              (`self.ClearDialogueProgress`)
              (`self.CloseDialogue`))))))))