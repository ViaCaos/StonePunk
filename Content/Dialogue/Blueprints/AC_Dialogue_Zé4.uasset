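; Dialogue component for an NPC shown as "Homem alto" (tall man), who questions the player in Portuguese and warns of a deadly horror below, "A Mãe".
; It overrides Dialogue, calling the parent, then switching on DialogueTreeIndex, with only tree 0 defined.
; Nested AddDialogue calls branch on the chosen option when their state is Pass Through.
; Each final line clears dialogue progress and closes the dialogue.
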(fn `Dialogue`
  (`parent.Dialogue`)
  (switch `int` (`self.DialogueTreeIndex`)
    (:`0`
      (bind (_state _optionindex) (`self.AddDialogue` "Homem alto" "O que está fazendo aqui?" (`|MakeArray` "Eu vou matar.... Acabar com isso" "O que vocês fazer aqui?" :!type "Text")))
      (switch `/Game/Dialogue/Blueprints/Enum_DialogueState` _state
        (:`NewEnumerator0`
          (switch `int` _optionindex
            (:`0`
              (bind (_state_2 _optionindex_2) (`self.AddDialogue` "Homem alto" "Você idiota? Vai morrer" (`|MakeArray` "Eu sei que consigo" "O que tem lá?" :!type "Text")))
              (switch `/Game/Dialogue/Blueprints/Enum_DialogueState` _state_2
                (:`NewEnumerator0`
                  (switch `int` _optionindex_2
                    (:`0`
                      (bind _state_3 (`self.AddDialogue` "Homem alto" "Burro, a coisa vai comer você vivo" (`|MakeArray` "Encerrar Dialogo" :!type "Text")))
                      (switch `/Game/Dialogue/Blueprints/Enum_DialogueState` _state_3
                        (:`NewEnumerator0`
                          (`self.ClearDialogueProgress`)
                          (`self.CloseDialogue`))))
                    (:`1`
                      (bind (_state_4 _optionindex_3) (`self.AddDialogue` "Homem alto" "A coisa horrenda, A Mãe de tudo isso" (`|MakeArray` "Voce já desceu?" "Eu deveria ir lá?" :!type "Text")))
                      (switch `/Game/Dialogue/Blueprints/Enum_DialogueState` _state_4
                        (:`NewEnumerator0`
                          (switch `int` _optionindex_3
                            (:`0`
                              (bind _state_5 (`self.AddDialogue` "Homem alto" "Não  atrevo a jogar minha vida fora..... Mais  que já joguei" (`|MakeArray` "Encerrar Dialogo" :!type "Text")))
                              (switch `/Game/Dialogue/Blueprints/Enum_DialogueState` _state_5
                                (:`NewEnumerator0`
                                  (`self.ClearDialogueProgress`)
                                  (`self.CloseDialogue`))))
                            (:`1`
                              (bind _state_6 (`self.AddDialogue` "Homem alto" "Você sabe resposta....Mas acredita nela?" (`|MakeArray` "Encerrar Diálogo" :!type "Text")))
                              (switch `/Game/Dialogue/Blueprints/Enum_DialogueState` _state_6
                                (:`NewEnumerator0`
                                  (`self.ClearDialogueProgress`)
                                  (`self.CloseDialogue`))))))))))))
            (:`1`
              (bind _state_7 (`self.AddDialogue` "Homem alto" "Eu proteger os que......aqui ficaram" (`|MakeArray` "Encerrar diálogo" :!type "Text")))
              (switch `/Game/Dialogue/Blueprints/Enum_DialogueState` _state_7
                (:`NewEnumerator0`
                  (`self.ClearDialogueProgress`)
                  (`self.CloseDialogue`))))))))))