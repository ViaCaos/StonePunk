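; NPC_Zé2 is an NPC that turns to face the player and opens its dialogue when interacted with.
; The Interact event stores the instigator and calls OpenDialogue on the ACDialogueZé2 component.
; Every Tick it computes a look-at rotation toward the first player's pawn and applies it with pitch zeroed, so the actor stays upright while turning.
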(event `self.Interact`
  (params (Instigator :type "Actor Object Reference"))
  (set `self.InteractInstigator` Instigator)
  (`/Game/Dialogue/Blueprints/AC_Dialogue.OpenDialogue` (`self.AC_Dialogue_Zé2`)))

(event `self.ReceiveTick`
  (params (DeltaSeconds :type "Float (single-precision)"))
  (`self.K2_SetActorRotation` (`KismetMathLibrary.MakeRotator` (.roll (`KismetMathLibrary.FindLookAtRotation` (`self.K2_GetActorLocation`) (`self.K2_GetActorLocation` (`GameplayStatics.GetPlayerPawn` 0)))) 0.0 (.yaw (`KismetMathLibrary.FindLookAtRotation` (`self.K2_GetActorLocation`) (`self.K2_GetActorLocation` (`GameplayStatics.GetPlayerPawn` 0)))))))

(fn `UserConstructionScript`
  (`parent.UserConstructionScript`))