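; Base NPC Blueprint that supports player interaction and conversations, with a floating character name and a voice sound.
; The Construction Script fills the name text from CharacterName, and SetInteractionState shows or hides it.
; BeginPlay assigns the voice clip and pauses it, and ConversationOpen plays it alongside a debug greeting print.
; ConversationClosed notifies the InteractInstigator that the conversation has ended.
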(event `self.ReceiveBeginPlay`
  (`AudioComponent.SetSound` (`self.Audio`) "/Game/Audio/Voz9.Voz9")
  (`AudioComponent.SetPaused` (`self.Audio`) true))

(event `/Game/Dialogue/Blueprints/BPI_Interactable.SetInteractionState`
  (params (CanShowInteract :type Boolean))
  (if CanShowInteract
    (`SceneComponent.SetVisibility` (`self.Text_CharacterName`) true false)
    (else
      (`SceneComponent.SetVisibility` (`self.Text_CharacterName`) false false))))

(event `/Game/Dialogue/Blueprints/BPI_Interactable.ConversationClosed`
  (message `/Game/Dialogue/Blueprints/BPI_Interactable.ConversationClosed` (`self.InteractInstigator`)))

(event `/Game/Dialogue/Blueprints/BPI_Interactable.ConversationOpen`
  (`KismetSystemLibrary.PrintString` "Hello")
  (`AudioComponent.Play` (`self.Audio`) 0.0))

(fn `UserConstructionScript`
  (`TextRenderComponent.K2_SetText` (`self.Text_CharacterName`) (`self.CharacterName`)))