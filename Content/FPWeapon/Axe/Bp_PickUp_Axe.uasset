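; Axe pickup actor that hands its static mesh to whatever interacts with it, then removes itself from the world.
; Interact calls the destroy event and returns the mesh, with a very short delay before the actor is destroyed.
; A separate Axe_Movement event plays or stops an embedded Actor Sequence based on a movement flag.
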(event `Destroy_Axe`
  (`KismetSystemLibrary.Delay` 0.01)
  (`self.K2_DestroyActor`))

(event `Axe_Movement`
  (params (Movement :type Boolean) (`Delta Time` :type "Float (double-precision)"))
  (bind _sequenceplayer (`ActorSequenceComponent.SequencePlayer` (`self.ActorSequence`)))
  (if Movement
    (`MovieSceneSequencePlayer.Play` _sequenceplayer)
    (else
      (`MovieSceneSequencePlayer.Stop` _sequenceplayer))))

(fn `Interact`
  (returns (Axe :type "StaticMesh Object Reference"))
  (`self.Destroy_Axe`)
  (return (`StaticMeshComponent.StaticMesh` (`self.StaticMesh`))))

(fn `UserConstructionScript`)